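; BP_Beam is a short-lived beam actor that plays a shot sound on spawn, then shrinks until it disappears.
; BeginPlay stores the actor's initial scale and plays the 2D sound.
; Tick subtracts a fixed amount from all scale axes each frame without using delta time, so lifetime depends on frame rate.
; The actor destroys itself once Y scale drops below zero, and it has no overlap or hit logic.
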(event `self.ReceiveBeginPlay`
  (set `self.BeamScale` (`self.GetActorScale3D`))
  (`GameplayStatics.PlaySound2D` "/Game/Sound/ショット.ショット" 1.0 1.0 0.0 null null))

(event `self.ReceiveTick`
  (params (DeltaSeconds :type "Float (single-precision)"))
  (bind _returnvalue (- (`self.BeamScale`) (0.5 0.5 0.5)))
  (`self.SetActorScale3D` _returnvalue)
  (bind _output_get (set `self.BeamScale` _returnvalue))
  (if (< (.y _output_get) 0.0)
    (`self.K2_DestroyActor`)))

(fn `UserConstructionScript`)
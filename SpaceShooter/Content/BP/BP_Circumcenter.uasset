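; BP_Circumcenter is an actor that marks the circumcenter of three active cursors.
; Each Tick it counts GameInstance cursors in the Add or Update state.
; With exactly three, it computes their circumcenter from the cursor list, converts that measured value to a position and moves there.
; It destroys itself after a short delay for any other count, or when the GameInstance's Second value reaches zero.
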(event `self.ReceiveBeginPlay`)

(event `self.ReceiveTick`
  (params (DeltaSeconds :type "Float (single-precision)"))
  (`self.TimeLimit`)
  (set `self.CursorCnt` 0)
  (set `self.SumPosition` (0.0 0.0))
  (bind _asspaceshooter_game_instance (`/Game/BP/BPL_Utility.GetGameInstanceRef`))
  (bind _cursorlist (`/Game/BP/SpaceShooterGameInstance.CursorList` _asspaceshooter_game_instance))
  (for _array_element _cursorlist
    (switch `string` (`.State_6_9422BEEE4B83BF5EEBF035B9CC72F4A4` (break `/Game/BP/F_CursorListElement` _array_element))
      (:`add`
        _)
      (:`update`
        _))
    (set `self.CursorCnt` (+ (`self.CursorCnt`) 1)))
  (if (== (`self.CursorCnt`) 3)
    (bind _circumcenter (`/Game/BP/BPL_Utility.GetCircumcenter` _cursorlist))
    (bind _vector (`/Game/BP/BPL_Utility.FromMeasuredValueToPosition` _circumcenter))
    (`self.K2_SetActorLocation` _vector)
    (else
      (`KismetSystemLibrary.Delay` 0.1)
      (`self.K2_DestroyActor`))))

(event `TimeLimit`
  (bind _asspaceshooter_game_instance (`/Game/BP/BPL_Utility.GetGameInstanceRef`))
  (if (== (`/Game/BP/SpaceShooterGameInstance.Second` _asspaceshooter_game_instance) 0)
    (`self.K2_DestroyActor` self)))

(fn `UserConstructionScript`)
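; Space shooter enemy that bounces around the Z=0 plane and awards score when destroyed.
; Tick sweeps it along a random initial direction, latching a speed boost once the game instance's Second reaches ten or below.
; Hits randomize speed and redirect it by mirroring the hit normal about its current direction.
; Any overlap triggers a delayed beam, explosion and sound, then updates game instance score and enemy count before destroying it.
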(event `self.ReceiveBeginPlay`
  (set `self.Normal Vector` (`KismetMathLibrary.MakeVector` (`KismetMathLibrary.RandomFloatInRange` 0.0 1.0) (`KismetMathLibrary.RandomFloatInRange` 0.0 1.0)))
  (bind _asspaceshooter_game_instance (`/Game/BP/BPL_Utility.GetGameInstanceRef`))
  (set `self.As Space Shooter Game Instance` _asspaceshooter_game_instance))

(event `self.ReceiveTick`
  (params (DeltaSeconds :type "Float (single-precision)"))
  (bind _speed (`self.Speed`))
  (bind _normal_vector (`self.Normal Vector`))
  (`|ExecutionSequence`
    (:`then_0`
      (if (<= (`/Game/BP/SpaceShooterGameInstance.Second` (`self.As Space Shooter Game Instance`)) 10)
        (set `self.isSpeedUp` true)))
    (:`then_1`
      (if (`self.isSpeedUp`)
        (bind _new_location (`self.NewLocation` _normal_vector (* _speed 2.5)))
        (`self.K2_SetActorLocation` _new_location true)
        (else
          (bind _new_location_2 (`self.NewLocation` _normal_vector _speed))
          (`self.K2_SetActorLocation` _new_location_2 true))))))

(event `self.ReceiveHit`
  (params (MyComp :type "PrimitiveComponent Object Reference") (Other :type "Actor Object Reference") (OtherComp :type "PrimitiveComponent Object Reference") (bSelfMoved :type Boolean) (HitLocation :type "Vector Structure") (HitNormal :type "Vector Structure") (NormalImpulse :type "Vector Structure") (Hit :type "HitResult Structure (by ref)"))
  (set `self.Speed` (`KismetMathLibrary.RandomFloatInRange` 5.0 7.0))
  (set `self.Normal Vector` (`KismetMathLibrary.MirrorVectorByNormal` HitNormal (`self.Normal Vector`))))

(event `self.ReceiveActorBeginOverlap`
  (params (OtherActor :type "Actor Object Reference"))
  (bind _returnvalue (`self.K2_GetActorLocation`))
  (`KismetSystemLibrary.Delay` 0.2)
  (`|SpawnActorFromClass` "/Game/BP/BP_Beam.BP_Beam_C" (`KismetMathLibrary.MakeTransform` _returnvalue (struct :`Roll` 90.0) (8.0 8.0 8.0)) "Undefined" "OverrideRootScale" null null)
  (`KismetSystemLibrary.Delay` 0.2)
  (`GameplayStatics.SpawnEmitterAtLocation` "/Game/StarterContent/Particles/P_Explosion.P_Explosion" _returnvalue (struct) (1.5 1.5 1.5))
  (`GameplayStatics.PlaySound2D` "/Game/Sound/爆発2.爆発2" 1.0 1.0 0.0 null null)
  (bind _asspaceshooter_game_instance (`/Game/BP/BPL_Utility.GetGameInstanceRef`))
  (set `/Game/BP/SpaceShooterGameInstance.Score` (+ (`/Game/BP/SpaceShooterGameInstance.Score` _asspaceshooter_game_instance) (`self.Score`)) _asspaceshooter_game_instance)
  (set `/Game/BP/SpaceShooterGameInstance.EnemyCnt` (- (`/Game/BP/SpaceShooterGameInstance.EnemyCnt` _asspaceshooter_game_instance) 1) _asspaceshooter_game_instance)
  (`self.K2_DestroyActor`))

(fn `NewLocation`
  (params (`Normal Vector` :type "Vector Structure") (Speed :type "Float (double-precision)"))
  (returns (`New Location` :type "Vector Structure"))
  (return (* (+ (`self.K2_GetActorLocation`) (* `Normal Vector` Speed)) (1.0 1.0 0.0))))

(fn `UserConstructionScript`)
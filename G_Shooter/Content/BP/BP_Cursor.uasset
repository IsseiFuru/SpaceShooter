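; BP_Cursor is a cursor actor that mirrors one entry of the Game Instance's CursorList, selected by its SectionID.
; Every Tick it checks that entry's state: Update converts the measured position and moves the actor there, while Remove destroys it after a short delay.
; A TimeLimit event, also run each Tick, destroys the cursor when the Game Instance's Second counter reaches zero.
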(event `self.ReceiveBeginPlay`)

(event `self.ReceiveTick`
  (params (DeltaSeconds :type "Float (single-precision)"))
  (`self.TimeLimit`)
  (bind _asg_shooter_game_instance (`/Game/BP/BPL_Utility.GetGameInstanceRef`))
  (bind (_state _position) (break `/Game/BP/F_CursorListElement` (`|GetArrayItem` (`/Game/BP/G-ShooterGameInstance.CursorList` _asg_shooter_game_instance) (`self.SectionID`))))
  (switch `string` _state
    (:`update`
      (bind _vector (`/Game/BP/BPL_Utility.FromMeasuredValueToPosition` _position))
      (`self.K2_SetActorLocation` _vector))
    (:`remove`
      (`KismetSystemLibrary.Delay` 0.1)
      (`self.K2_DestroyActor`))))

(event `TimeLimit`
  (bind _asg_shooter_game_instance (`/Game/BP/BPL_Utility.GetGameInstanceRef`))
  (if (== (`/Game/BP/G-ShooterGameInstance.Second` _asg_shooter_game_instance) 0)
    (`self.K2_DestroyActor` self)))

(fn `UserConstructionScript`)
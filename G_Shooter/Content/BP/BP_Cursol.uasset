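; BP_Cursol is a cursor actor that mirrors one entry of the game instance's CursolList, selected by SectionID.
; Each Tick it reads that entry's state: Update converts the stored measured position into world Y and Z and moves the actor there.
; Update also prints the actor's bounds center for debugging, while Remove destroys the actor after a short delay.
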(event `self.ReceiveBeginPlay`)

(event `self.ReceiveTick`
  (params (DeltaSeconds :type "Float (single-precision)"))
  (bind _asosc_game_instance (`/Game/BP/BPL_Utility.GetGameInstanceRef`))
  (bind (_state _position) (break `/Game/BP/F_CursolListElement` (`|GetArrayItem` (`/Game/BP/OscGameInstance.CursolList` _asosc_game_instance) (`self.SectionID`))))
  (switch `string` _state
    (:`update`
      (bind _position_2 (`/Game/BP/BPL_Utility.FromMeasuredValueToPosition` _position))
      (`self.K2_SetActorLocation` (`KismetMathLibrary.MakeVector` 0.0 (`KismetMathLibrary.BreakVector2D` _position_2) (`.Y` (`KismetMathLibrary.BreakVector2D` _position_2))))
      (`KismetSystemLibrary.PrintString` (`KismetStringLibrary.Concat_StrStr` (`KismetStringLibrary.Conv_DoubleToString` (.y (`self.GetActorBounds` false))) ", " (`KismetStringLibrary.Conv_DoubleToString` (.z (`self.GetActorBounds` false))))))
    (:`remove`
      (`KismetSystemLibrary.Delay` 0.1)
      (`self.K2_DestroyActor`))))

(fn `UserConstructionScript`)
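; BP_Enemy is a bouncing enemy that moves in the YZ plane and awards score when destroyed.
; It picks a random direction at BeginPlay and moves each tick with a swept SetActorLocation.
; Each hit mirrors the direction off the surface normal and rerolls the speed.
; Any overlap destroys it after a short delay, then updates the score and enemy count on the game instance.
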(event `self.ReceiveBeginPlay`
  (set `self.NormalVector` (`KismetMathLibrary.MakeVector` 0.0 (`KismetMathLibrary.RandomFloatInRange` -1.0 1.0) (`KismetMathLibrary.RandomFloatInRange` -1.0 1.0))))

(event `self.ReceiveTick`
  (params (DeltaSeconds :type "Float (single-precision)"))
  (bind (_returnvalue_x _returnvalue_y _returnvalue_z) (`KismetMathLibrary.BreakVector` (+ (`self.K2_GetActorLocation`) (* (* (`self.NormalVector`) (`self.Speed`)) DeltaSeconds))))
  (`self.K2_SetActorLocation` (`KismetMathLibrary.MakeVector` 0.0 _returnvalue_y _returnvalue_z) true))

(event `self.ReceiveHit`
  (params (MyComp :type "PrimitiveComponent Object Reference") (Other :type "Actor Object Reference") (OtherComp :type "PrimitiveComponent Object Reference") (bSelfMoved :type Boolean) (HitLocation :type "Vector Structure") (HitNormal :type "Vector Structure") (NormalImpulse :type "Vector Structure") (Hit :type "HitResult Structure (by ref)"))
  (set `self.Speed` (`KismetMathLibrary.RandomFloatInRange` 400.0 900.0))
  (set `self.NormalVector` (`KismetMathLibrary.MirrorVectorByNormal` (`self.NormalVector`) HitNormal)))

(event `self.ReceiveActorBeginOverlap`
  (params (OtherActor :type "Actor Object Reference"))
  (`KismetSystemLibrary.PrintString` "Overlap")
  (`KismetSystemLibrary.Delay` 0.2)
  (`self.K2_DestroyActor`)
  (bind _asg_shooter_game_instance (`/Game/BP/BPL_Utility.GetGameInstanceRef`))
  (set `/Game/BP/G-ShooterGameInstance.Score` (+ (`/Game/BP/G-ShooterGameInstance.Score` _asg_shooter_game_instance) (`self.Score`)) _asg_shooter_game_instance)
  (bind _output_get (set `/Game/BP/G-ShooterGameInstance.EnemyCnt` (- (`/Game/BP/G-ShooterGameInstance.EnemyCnt` _asg_shooter_game_instance) 1) _asg_shooter_game_instance))
  (`KismetSystemLibrary.PrintString` (`KismetStringLibrary.Conv_IntToString` _output_get)))

(fn `UserConstructionScript`)
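; BP_Circumcenter is an actor that marks the circumcenter of three cursors held in the game instance's CursolList.
; Each Tick counts cursors in the Add or Update state; at exactly three, it converts their circumcenter from measured values and moves itself to that point on the Y-Z plane.
; With any other count, it destroys itself after a short delay.
; A position-averaging calculation is left unused.
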(event `self.ReceiveBeginPlay`)

(event `self.ReceiveTick`
  (params (DeltaSeconds :type "Float (single-precision)"))
  (set `self.CursolCnt` 0)
  (set `self.SumPosition` (0.0 0.0))
  (bind _asg_shooter_game_instance (`/Game/BP/BPL_Utility.GetGameInstanceRef`))
  (bind _cursollist (`/Game/BP/G-ShooterGameInstance.CursolList` _asg_shooter_game_instance))
  (for _array_element _cursollist
    (switch `string` (`.State_6_9422BEEE4B83BF5EEBF035B9CC72F4A4` (break `/Game/BP/F_CursolListElement` _array_element))
      (:`add`
        _)
      (:`update`
        _))
    (set `self.CursolCnt` (+ (`self.CursolCnt`) 1)))
  (if (== (`self.CursolCnt`) 3)
    (bind _circumcenter (`/Game/BP/BPL_Utility.GetCircumcenter` _cursollist))
    (bind _position (`/Game/BP/BPL_Utility.FromMeasuredValueToPosition` _circumcenter))
    (`self.K2_SetActorLocation` (`KismetMathLibrary.MakeVector` 0.0 (`KismetMathLibrary.BreakVector2D` _position) (`.Y` (`KismetMathLibrary.BreakVector2D` _position))))
    (else
      (`KismetSystemLibrary.Delay` 0.1)
      (`self.K2_DestroyActor`))))

(fn `UserConstructionScript`)